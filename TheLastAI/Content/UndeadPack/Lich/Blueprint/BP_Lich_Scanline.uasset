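; Lich enemy character for a top-down game that melee-attacks the player and credits kills to them.
; On spawn it randomizes yaw, applies a dynamic dissolve material and delays AI controller logic by distance from world origin, staggering activation.
; An overlap box gates Attack, which times fixed damage to the player's health component from montage length.
; Death triggers animation and Niagara effect, unpossesses, then destroys the actor.
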(event OnComponentBeginOverlap(AttackBox)
  (params (OverlappedComponent :type Primitive%20Component%20Object%20Reference) (OtherActor :type Actor%20Object%20Reference) (OtherComp :type Primitive%20Component%20Object%20Reference) (OtherBodyIndex :type Integer) (bFromSweep :type Boolean) (SweepResult :type Hit%20Result%20Structure%20%28by%20ref%29))
  (Variables|Default|SetbCanAttack true))

(event OnComponentEndOverlap(AttackBox)
  (params (OverlappedComponent :type Primitive%20Component%20Object%20Reference) (OtherActor :type Actor%20Object%20Reference) (OtherComp :type Primitive%20Component%20Object%20Reference) (OtherBodyIndex :type Integer))
  (Variables|Default|SetbCanAttack false))

(event Custom|Go%20To%20Player
  (bind _asaicontroller (Utilities|Casting|CastToAIController (Pawn|GetController)))
  (AI|AIMoveTo _asaicontroller "0, 0, 0" (Game|Player|GetPlayerPawn 0) -1.0 "Enable" "Enable" true true
    (:then
      (Utilities|FlowControl|Delay 5.0))))

(event Custom|Attack
  (if (Variables|Default|GetbCanAttack)
    (Variables|Default|SetbIsAttacking true)
    (bind _returnvalue (Animation|PlayAnimMontage "/Game/UndeadPack/Lich/Animations/AM_Attack.AM_Attack" 2.0 (Utilities|String|StringToName (Utilities|String|ToString(Integer) (Math|Random|RandomInteger 1)))))
    (Audio|PlaySoundatLocation "/Game/MilitaryWeapSilver/Sound/Rifle/Cues/RifleA_Fire_Cue.RifleA_Fire_Cue" (Transformation|GetWorldLocation (Variables|Collision|GetCapsuleComponent)) "0, 0, 0" 1.0 1.0 0.0 0 0 0 0)
    (Utilities|FlowControl|Delay (/ _returnvalue 1e+01))
    (bind _asbp_top_down_wasdcharacter (Utilities|Casting|CastToBP_TopDownWASDCharacter (Game|Player|GetPlayerPawn 0)))
    (Default|Damage (Variables|/Game/TopDownWASD/Blueprints/BP_TopDownWASDCharacter.BP_TopDownWASDCharacter_C|GetBP_Health_Comp _asbp_top_down_wasdcharacter) 1e+01)
    (Utilities|FlowControl|Delay (/ _returnvalue 1e+01))
    (Animation|StopAnimMontage "/Game/UndeadPack/Lich/Animations/AM_Attack.AM_Attack")
    (Variables|Default|SetbIsAttacking false)))

(event EventDeath
  (params (DamageCauser :type Actor%20Object%20Reference))
  (bind _asbp_top_down_wasdcharacter (Utilities|Casting|CastToBP_TopDownWASDCharacter DamageCauser))
  (Default|AddKilling _asbp_top_down_wasdcharacter)
  (bind _asabp_lich (Utilities|Casting|CastToABP_Lich (Components|SkeletalMesh|GetAnimInstance (Variables|Character|GetMesh))))
  (Default|Die _asabp_lich)
  (Components|Activation|Activate (Variables|Default|GetNS_Death) false)
  (Pawn|UnPossess (Pawn|GetController))
  (Utilities|FlowControl|Delay 3.0)
  (Actor|DestroyActor))

(event EventBeginPlay
  (Transformation|SetActorRotation (Math|Rotator|MakeRotator 0.0 0.0 (Math|Random|RandomFloatinRange 0.0 3.6e+02)) true)
  (bind _returnvalue (Rendering|Material|CreateDynamicMaterialInstance (Variables|Default|GetMaterialDissolve) "None" "None" :!class /Script/Engine.KismetMaterialLibrary))
  (bind _output_get (Variables|Default|SetMaterial%20Instance _returnvalue))
  (Rendering|Material|SetMaterial (Variables|Character|GetMesh) 0 _output_get)
  (Utilities|FlowControl|Delay (/ (Math|Vector|Distance(Vector) "0, 0, 0" (Transformation|GetActorLocation)) 1e+03))
  (bind _asbp_enemy_aicontroller (Utilities|Casting|CastToBP_EnemyAIController (Pawn|GetController)))
  (Default|StartLogic _asbp_enemy_aicontroller))

(fn ConstructionScript)

(fn GetCanAttack
  (return (Variables|Default|GetbCanAttack)))

(fn GetIsAttacking
  (return (Variables|Default|GetbIsAttacking)))