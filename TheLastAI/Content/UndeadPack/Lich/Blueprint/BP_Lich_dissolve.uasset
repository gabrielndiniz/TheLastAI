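; BP_Lich_dissolve is a Lich Blueprint that continuously animates a dissolve effect on its mesh.
; BeginPlay applies a dynamic instance of the dissolve material, with random starting dissolve and edge emissive values and a fixed edge width.
; Tick ping-pongs both values between their min and max by flipping each step's sign at the limits, scales movement by delta time, and writes them to the material.
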(event EventTick
  (params (DeltaSeconds :type Float%20%28single-precision%29))
  (Variables|Default|SetDelta%20Seconds DeltaSeconds)
  (Utilities|FlowControl|Sequence
    (:then_0
      (if (>= (Variables|Default|GetCurrentEmissive) (Variables|Default|GetMaxEmissive))
        (Variables|Default|SetStepEmissive (* (Variables|Default|GetStepEmissive) -1.0) :!label _label)
        (elif (>= (Variables|Default|GetMinEmissive) (Variables|Default|GetCurrentEmissive))
          (goto _label))))
    (:then_1
      (if (>= (Variables|Default|GetCurrentDissolve) (Variables|Default|GetMaxDissolve))
        (Variables|Default|SetStepDissolve (* (Variables|Default|GetStepDissolve) -1.0) :!label _label_2)
        (elif (>= (Variables|Default|GetMinDissolve) (Variables|Default|GetCurrentDissolve))
          (goto _label_2))))
    (:then_2
      (Variables|Default|SetCurrentEmissive (+ (Variables|Default|GetCurrentEmissive) (* (Variables|Default|GetStepEmissive) (Variables|Default|GetDelta%20Seconds))))
      (Variables|Default|SetCurrentDissolve (+ (Variables|Default|GetCurrentDissolve) (* (Variables|Default|GetStepDissolve) (Variables|Default|GetDelta%20Seconds)))))
    (:then_3
      (Rendering|Material|SetScalarParameterValue (Variables|Default|GetMaterial%20Instance) "Dissolve" (Variables|Default|GetCurrentDissolve) :!class /Script/Engine.MaterialInstanceDynamic)
      (Rendering|Material|SetScalarParameterValue (Variables|Default|GetMaterial%20Instance) "Dissolve Edge Emissive" (Variables|Default|GetCurrentEmissive) :!class /Script/Engine.MaterialInstanceDynamic))))

(event EventBeginPlay
  (bind _returnvalue (Rendering|Material|CreateDynamicMaterialInstance (Variables|Default|GetMaterialDissolve) "None" "None" :!class /Script/Engine.KismetMaterialLibrary))
  (bind _output_get (Variables|Default|SetMaterial%20Instance _returnvalue))
  (Rendering|Material|SetMaterial (Variables|Character|GetMesh) 0 _output_get)
  (Variables|Default|SetCurrentDissolve (+ (* (Math|Random|RandomFloat) (- (Variables|Default|GetMaxDissolve) (Variables|Default|GetMinDissolve))) (Variables|Default|GetMinDissolve)))
  (Variables|Default|SetCurrentEmissive (+ (* (Math|Random|RandomFloat) (- (Variables|Default|GetMaxEmissive) (Variables|Default|GetMinEmissive))) (Variables|Default|GetMinEmissive)))
  (Rendering|Material|SetScalarParameterValue (Variables|Default|GetMaterial%20Instance) "Dissolve" (Variables|Default|GetCurrentDissolve) :!class /Script/Engine.MaterialInstanceDynamic)
  (Rendering|Material|SetScalarParameterValue (Variables|Default|GetMaterial%20Instance) "Dissolve Edge Emissive" (Variables|Default|GetCurrentEmissive) :!class /Script/Engine.MaterialInstanceDynamic)
  (Rendering|Material|SetScalarParameterValue (Variables|Default|GetMaterial%20Instance) "Dissolve Edge Width" 0.2 :!class /Script/Engine.MaterialInstanceDynamic))

(fn ConstructionScript)