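; BP_LaserGun is a laser weapon that damages enemies at a rate set by DamagePerSecond.
; Construction snaps the Barrel to the Gun socket and configures BPPointingLaser's effects and range.
; Shoot rotates the Barrel from the Direction point and triggers the laser; StopShoot stops it.
; Hits on EnemyHealth-tagged health components deal damage in interval-sized chunks, gated by a Tick countdown, and print the owner's name.
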(event EventBeginPlay)

(event Collision|EventActorBeginOverlap
  (params (OtherActor :type Actor%20Object%20Reference)))

(event EventTick
  (params (DeltaSeconds :type Float%20%28single-precision%29))
  (if (> (Variables|Default|GetLast%20Time%20Damaged) 0.0)
    (Variables|Default|SetLast%20Time%20Damaged (Math|Float|Clamp(Float) (- (Variables|Default|GetLast%20Time%20Damaged) DeltaSeconds) 0.0 (Variables|Default|GetTime%20Considered%20To%20Damage)))))

(fn ConstructionScript
  (Transformation|AttachComponentToComponent (Variables|Default|GetBarrel) (Variables|Default|GetGun) "Connection" "SnapToTarget" "KeepRelative" "KeepRelative" false)
  (Default|SetParameters (Variables|Default|GetBP_PointingLaser) (Variables|Default|GetNSLaserPointing) (Variables|Default|GetNSLaserImpact) (Variables|Default|GetLaser%20Distance)))

(fn Shoot
  (params (Direction :type Vector))
  (bind _returnvalue (Components|GetOwner))
  (bind _barrel (Variables|Default|GetBarrel))
  (bind _returnvalue_2 (Transformation|GetWorldLocation _barrel))
  (bind _returnvalue_3 (Math|Rotator|FindLookatRotation Direction _returnvalue_2))
  ;[1 1 1] Barrel Pointing at front of character
  (Transformation|SetWorldRotation _barrel (Math|Rotator|MakeRotator (+ (.roll _returnvalue_3) 9e+01) (.pitch _returnvalue_3) (+ (.yaw _returnvalue_3) -9e+01)) false false)
  (bind _hit_actor (Default|Trigger (Variables|Default|GetBP_PointingLaser)))
  (Utilities|IsValid (Class|Actor|FindComponentbyTag _hit_actor "/Game/CloseCombat/Blueprints/Player/Components/BP_Health_Comp.BP_Health_Comp_C" "EnemyHealth")
    (:Is%20Valid
      (if (< (Variables|Default|GetLast%20Time%20Damaged) 0.0001)
        (Variables|Default|SetLast%20Time%20Damaged (Variables|Default|GetTime%20Considered%20To%20Damage))
        (Default|Damage (Class|Actor|FindComponentbyTag _hit_actor "/Game/CloseCombat/Blueprints/Player/Components/BP_Health_Comp.BP_Health_Comp_C" "EnemyHealth") (* (Variables|Default|GetDamage%20per%20Second) (Variables|Default|GetTime%20Considered%20To%20Damage)) _returnvalue)
        (Development|PrintString (Utilities|GetDisplayName _returnvalue))))))

(fn StopShoot
  (Default|StopTrigger (Variables|Default|GetBP_PointingLaser)))